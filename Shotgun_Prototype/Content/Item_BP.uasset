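; Item_BP is a networked weapon item with magazine and reserve ammo, server-side firing and timed reloading.
; FireWeapon checks cooldown, reload state and ammo, spends a round, damages hits from a multi sphere trace that ignores the shooter's pawn, then starts the fire-rate cooldown.
; Firing also spawns muzzle emitters and sends an OSC message to an external target.
; Reloading waits out a delay, then tops up the magazine from reserve ammo.
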(event Custom|ReloadWeapon
  ;[1 0.6539 0.3559] Server-Side Reload Function
  (if (< (Variables|Default|GetShotsInMagazine) (Variables|Default|GetMagazineSize))
    (Variables|Default|SetIsReloading true)
    (Utilities|FlowControl|Delay (Variables|Default|GetReloadTime))
    (Variables|Default|SetIsReloading false)
    (CallFunction|ReloadWeaponFunc)))

(event Custom|Destroy%20Self
  (Actor|DestroyActor))

(event Custom|ServerFire_CapsuleTrace
  (params (ClientEyePos :type Vector) (ClientEyeRot :type Rotator) (Instigator :type Controller%20Object%20Reference))
  (bind _returnvalue (Math|Vector|GetForwardVector ClientEyeRot))
  (bind _spread (Variables|Default|GetSpread))
  ;[1 0.6539 0.3559] Server-Side Logic for handling hit detection
  (bind _outhits (Class|KismetSystemLibrary|SphereTraceMultiNEW (+ ClientEyePos (* _returnvalue _spread)) (+ ClientEyePos (* _returnvalue (Variables|Default|GetRange))) _spread "TraceTypeQuery2" false (Utilities|Array|MakeArray (Pawn|GetControlledPawn Instigator)) "Persistent" true))
  (for _array_element _outhits
    (Game|Damage|ApplyDamage (.HitActor (Collision|BreakHitResult _array_element)) (Variables|Default|GetBaseDamage) Instigator 0)
    (Development|PrintString (Utilities|String|Append "capsule trace hit " (Utilities|GetDisplayName (.HitActor (Collision|BreakHitResult _array_element)))))))

(event Custom|FireWeapon_Effects
  (bind _objectmesh (Variables|Default|GetObjectMesh))
  (bind _returnvalue (Transformation|GetSocketTransform _objectmesh "Muzzle" "RTS_World"))
  (bind (_location _rotation) (Math|Transform|BreakTransform _returnvalue))
  (Effects|SpawnEmitteratLocation "/Game/StarterContent/Particles/P_Explosion.P_Explosion" _location)
  (Effects|SpawnEmitteratLocation "/Game/StarterContent/Particles/ShotgunFlak.ShotgunFlak" _location _rotation)
  (Class|OscFunctionLibrary|SendOsc "/player/guns"))

(event Custom|ActivateFirerateCooldown
  ;[1 1 1] Trigger Weapon's Firerate Cooldown (Sets Replicated Variable)
  (Variables|Default|SetIsOnFireCooldown true)
  (Utilities|FlowControl|Delay (Variables|Default|GetFireRate))
  (Variables|Default|SetIsOnFireCooldown false))

(event Custom|FireWeapon
  (params (Origin :type Vector) (Rotation :type Rotator) (Instigator :type Controller%20Object%20Reference))
  ;[1 0.6539 0.3559] Server-Side Fire Weapon
  (if (not (Variables|Default|GetIsOnFireCooldown))
    (if (not (Variables|Default|GetIsReloading))
      (if (> (Variables|Default|GetShotsInMagazine) 0)
        (CallFunction|ReduceAmmo)
        (CallFunction|ServerFireCapsuleTrace Origin Rotation Instigator)
        (CallFunction|FireWeaponEffects)
        (CallFunction|ActivateFirerateCooldown)))))

(fn ConstructionScript)

(fn ReduceAmmo
  (bind _shotsinmagazine (Variables|Default|GetShotsInMagazine))
  (if (> _shotsinmagazine 0)
    (Math|Integer|DecrementInt _shotsinmagazine
      (:%20%20
        (return)))))

(fn ReloadWeaponFunc
  (bind _output_get (LocalVariables|SetRoomInMag (- (Variables|Default|GetMagazineSize) (Variables|Default|GetShotsInMagazine))))
  ;[1 1 1] If we have enough ammo to fully refil, do it
  (if (>= (Variables|Default|GetCurrentAmmo) _output_get)
    ;;[1 1 1] Reduce Current Ammo
    (Variables|Default|SetCurrentAmmo (- (Variables|Default|GetCurrentAmmo) _output_get))
    ;;[1 1 1] Fill Magazine
    (Variables|Default|SetShotsInMagazine (+ (Variables|Default|GetShotsInMagazine) _output_get))
    (else
      ;[1 1 1] If we don't have enough ammo to fully refill, dump in what we have and set current ammo to 0
      (Variables|Default|SetShotsInMagazine (+ (Variables|Default|GetShotsInMagazine) (Variables|Default|GetCurrentAmmo)))
      (Variables|Default|SetCurrentAmmo 0)))
  (return))

(fn OnRepHasOwner)