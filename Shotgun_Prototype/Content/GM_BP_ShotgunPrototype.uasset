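; Game mode for the shotgun prototype, running teams, lives, spawning, scoring and server travel to arenas.
; InitializeTeams deals players round-robin into teams, sets lives and builds scoreboards; -1 means free-for-all or infinite lives.
; Server spawn events possess pawns at random team-matched starts; respawns check lives and report exhausted players to the game state, though CheckCanRespawn zeroes remaining lives.
; A shot-frequency counter rises per shot and decays on Tick.
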(event Custom|Initialize%20Teams
  (bind _returnvalue (Game|GetGameState))
  (bind _playerarray (Variables|/Script/Engine.GameState|GetPlayerArray _returnvalue))
  ;[1 1 1] Intialize Team Logic
  (bind _asgs_bp_prototype (Utilities|Casting|CastToGS_BP_Prototype _returnvalue))
  (Default|GetAllPlayers _asgs_bp_prototype)
  (for (_array_element _array_index) _playerarray
    (bind _teamnum (CallFunction|GetTeam _array_index (Variables|Default|GetNumTeams)))
    (bind _asps_bp_prototype (Utilities|Casting|CastToPS_BP_Prototype _array_element))
    (bind _output_get (Variables|/Game/PS_BP_Prototype.PS_BP_Prototype_C|SetTeam _asps_bp_prototype _teamnum))
    (Default|AddtoTeamArray _asgs_bp_prototype _output_get _asps_bp_prototype)
    (Variables|/Game/PS_BP_Prototype.PS_BP_Prototype_C|SetLivesRemaining _asps_bp_prototype (Variables|Default|GetNumLives))
    (Utilities|Casting|CastToPC_BP_Prototype (Components|GetOwner _asps_bp_prototype)))
  ;;[1 1 1] Intialize ScoreBoard
  (for _array_element_2 _playerarray
    (bind _asps_bp_prototype_2 (Utilities|Casting|CastToPS_BP_Prototype _array_element_2))
    (bind _aspc_bp_prototype (Utilities|Casting|CastToPC_BP_Prototype (Components|GetOwner _asps_bp_prototype_2)))
    (Default|InitializeScoreboard _aspc_bp_prototype)))

(event Custom|SpawnPawnAtSpawnPoint_Server
  (params (Controller :type Controller%20Object%20Reference) (SpawnAs :type Pawn%20Class%20Reference))
  ;[1 1 1] Spawn Pawn at Spawn Point
  (Utilities|IsValid Controller
    (:Is%20Valid
      (Networking|SwitchHasAuthority
        (:Authority
          (bind _asps_bp_prototype (Utilities|Casting|CastToPS_BP_Prototype (Variables|/Script/Engine.Controller|GetPlayerState Controller)))
          (bind _outactors (Actor|GetAllActorsOfClass "/Game/Blueprints/BP_PlayerStart.BP_PlayerStart_C"))
          (bind _spawn_point (CallFunction|GetSpawnPoints (Variables|/Game/PS_BP_Prototype.PS_BP_Prototype_C|GetTeam _asps_bp_prototype) _outactors (Variables|Default|GetNumTeams)))
          (CallFunction|SpawnPawnServer SpawnAs (Transformation|GetActorTransform _spawn_point) Controller))))))

(event Custom|Spawn%20Players
  ;[1 1 1] Intialize Players at Start of Match
  (for _array_element (Variables|/Script/Engine.GameState|GetPlayerArray (Game|GetGameState))
    (bind _asps_bp_prototype (Utilities|Casting|CastToPS_BP_Prototype _array_element))
    (bind _aspc_bp_prototype (Utilities|Casting|CastToPC_BP_Prototype (Components|GetOwner _asps_bp_prototype)))
    (Utilities|IsValid (Pawn|GetControlledPawn _aspc_bp_prototype)
      (:Is%20Valid
        (Actor|DestroyActor (Pawn|GetControlledPawn _aspc_bp_prototype)))
      (:Is%20Not%20Valid
        _))
    (CallFunction|SpawnPawnatSpawnPointServer _aspc_bp_prototype "/Game/GladiatorStuff/Gladiator_BP.Gladiator_BP_C")))

(event Custom|Destroy%20Pawn
  (params (Pawn :type Pawn%20Object%20Reference))
  ;[1 1 1] Original Respawn Logic
  (Utilities|IsValid Pawn
    (:Is%20Valid
      (Actor|DestroyActor Pawn))))

(event Custom|Respawn
  (params (PlayerController :type Player%20Controller%20Object%20Reference) (RespawnAs :type Pawn%20Class%20Reference) (Delay :type Boolean))
  (bind _playerstate (Variables|/Script/Engine.Controller|GetPlayerState PlayerController))
  ;[1 1 1] Original Respawn Logic
  (bind _asps_bp_prototype (Utilities|Casting|CastToPS_BP_Prototype _playerstate))
  (bind (_new_lives _can_respawn) (CallFunction|CheckLives (Variables|/Game/PS_BP_Prototype.PS_BP_Prototype_C|GetLivesRemaining _asps_bp_prototype)))
  (Variables|/Game/PS_BP_Prototype.PS_BP_Prototype_C|SetLivesRemaining _asps_bp_prototype _new_lives)
  (if _can_respawn
    (if Delay
      (Utilities|FlowControl|Delay (Variables|Default|GetRespawn%20Delay)))
    (Utilities|IsValid PlayerController
      (:Is%20Valid
        (Networking|SwitchHasAuthority
          (:Authority
            (bind _asps_bp_prototype_2 (Utilities|Casting|CastToPS_BP_Prototype _playerstate))
            (bind _outactors (Actor|GetAllActorsOfClass "/Game/Blueprints/BP_PlayerStart.BP_PlayerStart_C"))
            (bind _spawn_point (CallFunction|GetSpawnPoints (Variables|/Game/PS_BP_Prototype.PS_BP_Prototype_C|GetTeam _asps_bp_prototype_2) _outactors (Variables|Default|GetNumTeams)))
            (bind _returnvalue (Game|SpawnActorfromClass RespawnAs (Transformation|GetActorTransform _spawn_point) "Undefined" PlayerController 0))
            (Utilities|IsValid _returnvalue
              (:Is%20Valid
                (Pawn|Possess PlayerController _returnvalue)))))))
    (else
      (bind _asgs_bp_prototype (Utilities|Casting|CastToGS_BP_Prototype (Game|GetGameState)))
      (Default|Die _asgs_bp_prototype _asps_bp_prototype))))

(event Custom|SpawnPawnOnDelay_Server
  (params (SpawnDelay :type Float%20%28single-precision%29) (Controller :type Controller%20Object%20Reference) (Pawn%20Class :type Pawn%20Class%20Reference))
  ;[1 1 1] Spawn Pawn w/ Delay
  (Utilities|FlowControl|Delay SpawnDelay)
  (CallFunction|SpawnPawnatSpawnPointServer Controller Pawn%20Class))

(event Custom|AddScore
  (params (Damage%20Causer :type Controller%20Object%20Reference))
  ;[1 1 1] Add Score
  (bind _asps_bp_prototype (Utilities|Casting|CastToPS_BP_Prototype (Variables|/Script/Engine.Controller|GetPlayerState Damage%20Causer))
    (:then
      (Default|AddScore _asps_bp_prototype 1 (Variables|/Game/PS_BP_Prototype.PS_BP_Prototype_C|GetTeam _asps_bp_prototype)))
    (:CastFailed
      (Development|PrintString "Cast to PS_BP_Prototype Failed" true true "(R=1.000000,G=0.000000,B=0.000000,A=1.000000)" 5e+02))))

(event Custom|Move%20to%20Arena
  (params (Map%20Name :type String))
  (if (Ability|HasAuthority (Game|GetGameMode))
    (Development|ExecuteConsoleCommand (Utilities|String|Append "servertravel " Map%20Name) (Game|GetPlayerController 0))))

(event Custom|PlayerShot
  (Variables|Default|SetShotFrequency (+ (Variables|Default|GetShotFrequency) 1.0)))

(event Custom|CheckCanRespawn
  (params (RequestingController :type Controller%20Object%20Reference))
  ;[1 1 1] Check if Able to Assign New Pawn to Controller
  (bind _asps_bp_prototype (Utilities|Casting|CastToPS_BP_Prototype (Variables|/Script/Engine.Controller|GetPlayerState RequestingController)))
  (bind _can_respawn (CallFunction|CheckLives (Variables|/Game/PS_BP_Prototype.PS_BP_Prototype_C|GetLivesRemaining _asps_bp_prototype)))
  (Variables|/Game/PS_BP_Prototype.PS_BP_Prototype_C|SetLivesRemaining _asps_bp_prototype 0)
  (if _can_respawn
    (CallFunction|SpawnPawnonDelayServer (Variables|Default|GetRespawn%20Delay) RequestingController "/Game/GladiatorStuff/Gladiator_BP.Gladiator_BP_C")
    (else
      (bind _asgs_bp_prototype (Utilities|Casting|CastToGS_BP_Prototype (Game|GetGameState)))
      (Default|Die _asgs_bp_prototype _asps_bp_prototype))))

(event Custom|SpawnPawn_Server
  (params (Spawn%20As :type Pawn%20Class%20Reference) (SpawnLocation :type Transform) (Controller :type Controller%20Object%20Reference))
  ;[1 1 1] Spawn Pawn and Assign Controller
  (Utilities|IsValid (Pawn|GetControlledPawn Controller)
    (:Is%20Valid
      (Pawn|UnPossess Controller))
    (:Is%20Not%20Valid
      _))
  (bind _returnvalue (Game|SpawnActorfromClass Spawn%20As SpawnLocation "AdjustIfPossibleButDontSpawnIfColliding" Controller 0))
  (Utilities|IsValid _returnvalue
    (:Is%20Valid
      (Pawn|Possess Controller _returnvalue))))

(event EventBeginPlay
  ;[1 1 1] Initialize Match
  (bind _asgs_bp_prototype (Utilities|Casting|CastToGS_BP_Prototype (Game|GetGameState)))
  (Default|SetMatchState _asgs_bp_prototype "NewEnumerator3")
  (bind _asps_bp_prototype (Utilities|Casting|CastToPS_BP_Prototype (Variables|/Script/Engine.Controller|GetPlayerState (Game|GetPlayerController 0)))))

(event EventTick
  (params (DeltaSeconds :type Float%20%28single-precision%29))
  (Variables|Default|SetShotFrequency (Math|Float|Clamp(Float) (- (Variables|Default|GetShotFrequency) DeltaSeconds) 0.0 1e+01)))

(fn ConstructionScript)

(fn GetSpawnPoints
  (params (Team :type Integer) (Spawn%20Points :type Array%20of%20BP%20Player%20Start%20Object%20References) (NumTeams :type Integer))
  (bind _team_spawns (LocalVariables|GetTeam%20Spawns))
  (switch int NumTeams
    (:Default
      (for _array_element Spawn%20Points
        (if (== (Variables|/Game/Blueprints/BP_PlayerStart.BP_PlayerStart_C|GetTeam _array_element) Team)
          (Utilities|Array|AddUnique (LocalVariables|GetTeam%20Spawns) _array_element)))
      (return (Utilities|Array|Get(acopy) _team_spawns (Math|Random|RandomInteger (Utilities|Array|Length _team_spawns)))))
    (:-1
      (return (Utilities|Array|Get(acopy) Spawn%20Points (Math|Random|RandomInteger (Utilities|Array|Length Spawn%20Points)))))))

(fn CheckLives
  (params (Current%20Lives :type Integer))
  (switch int Current%20Lives
    (:Default
      (bind _result (Math|Integer|DecrementInt Current%20Lives)
        (:%20%20
          (return _result true))))
    (:-1
      (return Current%20Lives true))
    (:0
      (return Current%20Lives false))))

(fn GetTeam
  (params (PlayerNum :type Integer) (NumTeams :type Integer))
  (switch int NumTeams
    (:Default
      (return (Math|Integer|%(Integer) PlayerNum NumTeams)))
    (:-1
      (return PlayerNum))))