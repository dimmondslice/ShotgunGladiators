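; Prototype player controller that owns the HUD and in-game menu and forwards movement axes to the possessed Gladiator pawn.
; The menu toggle switches visibility, input mode and mouse cursor together.
; Session host, find, join and exit events delegate to the game instance.
; Respawn destroys the pawn, then asks the game mode on authority for a delayed respawn, while other events add score through player state and print the player count.
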(event Custom|RespawnPlayer
  (params (Delay :type Boolean))
  ;[1 1 1] Respawn Logic
  ;;[0.2351 0.6742 1] Command to Respawn the Player -> Will request from Server
  (Utilities|IsValid (Pawn|GetControlledPawn self)
    (:Is%20Valid
      (CallFunction|DestroyPawn))
    (:Is%20Not%20Valid
      _))
  (CallFunction|RequestRespawn Delay))

(event Custom|Destroy%20Pawn
  ;[1 1 1] Respawn Logic
  ;;[1 0.6539 0.3559] Server-side Destroy Pawn Event
  (Actor|DestroyActor (Pawn|GetControlledPawn)))

(event Custom|JoinSession_Event
  (params (SelectedSession :type Blueprint%20Session%20Result%20Structure))
  ;[1 1 1] Handle Sessions via Game Instance
  ;;[1 0.6539 0.3559] Send Command to Game Instance to Join an Available Session
  (bind _asgi_sggprototype (Utilities|Casting|CastToGI_SGGPrototype (Game|GetGameInstance))
    (:then
      (Default|GIJoinLobby _asgi_sggprototype self SelectedSession))
    (:CastFailed
      (Development|PrintString "Error: Cast To Game Instance Failed" true true "(R=1.000000,G=0.188499,B=0.000000,A=1.000000)"))))

(event Custom|Create%20HUD
  (bind _returnvalue (UserInterface|CreateWidget "/Game/HUD.HUD_C" self))
  (bind _output_get (Variables|Default|SetHUD _returnvalue))
  (UserInterface|Viewport|AddtoViewport _output_get 0))

(event Custom|ExitSession_Event
  ;[1 1 1] Handle Sessions via Game Instance
  (bind _asgi_sggprototype (Utilities|Casting|CastToGI_SGGPrototype (Game|GetGameInstance))
    (:then
      (Default|GIExitSession _asgi_sggprototype self))
    (:CastFailed
      (Development|PrintString "Error: Cast To Game Instance Failed" true true "(R=1.000000,G=0.188499,B=0.000000,A=1.000000)"))))

(event Custom|AddScore
  (params (Damage%20Causer :type Controller%20Object%20Reference))
  ;[1 1 1] Add Score - Server Bound
  (bind _asps_bp_prototype (Utilities|Casting|CastToPS_BP_Prototype (Variables|/Script/Engine.Controller|GetPlayerState Damage%20Causer))
    (:then
      (Default|AddScore _asps_bp_prototype 1))
    (:CastFailed
      (Development|PrintString "Cast to PS_BP_Prototype Failed" true true "(R=1.000000,G=0.000000,B=0.000000,A=1.000000)" 5e+02))))

(event Custom|GetListOfPlayers_Server
  (CallFunction|PrinttoClient (Utilities|Array|Length (Variables|/Script/Engine.GameState|GetPlayerArray (Game|GetGameState)))) ; Send Number of Players the Server reported to the Client who asked
)

(event Custom|FindSessions_Event
  ;[1 1 1] Handle Sessions via Game Instance
  ;;[1 1 1] Send Command to Game Instance to FInd Available Sessions
  (bind _asgi_sggprototype (Utilities|Casting|CastToGI_SGGPrototype (Game|GetGameInstance))
    (:then
      (Default|GIFindLobbies _asgi_sggprototype self))
    (:CastFailed
      (Development|PrintString "Error: Cast To Game Instance Failed" true true "(R=1.000000,G=0.188499,B=0.000000,A=1.000000)"))))

(event Custom|PrintToClient
  (params (Num%20of%20Players :type Integer))
  (Development|PrintString (Utilities|String|ToString(Integer) Num%20of%20Players) true true "(R=0.000000,G=1.000000,B=0.988496,A=1.000000)"))

(event Custom|SetInGameMenuVisibility_Event
  (params (VisibilitySetting :type ESlateVisibility%20Enum))
  ;[1 1 1] UI: Logic for Opening and closing In-Game Menu
  ;;[0.2351 0.6742 1] Event for Setting In-Game Menu Visibility from Outside Class
  (CallFunction|SetinGameMenuVisibility (Variables|Default|GetW_TravelMenu) VisibilitySetting))

(event Custom|RequestRespawn
  (params (Delay :type Boolean))
  (bind _returnvalue (Game|GetGameMode))
  ;[1 1 1] Respawn Logic
  ;;[1 0.6539 0.3559] Server Request to Respawn Pawn for Owning Controller
  (Networking|SwitchHasAuthority
    (:Authority
      (Utilities|IsValid _returnvalue
        (:Is%20Valid
          (bind _asgm_bp_shotgun_prototype (Utilities|Casting|CastToGM_BP_ShotgunPrototype _returnvalue))
          (Utilities|IsValid _asgm_bp_shotgun_prototype
            (:Is%20Valid
              (bind _returnvalue_2 (Utilities|Casting|CastToPlayerController self))
              (Default|Respawn _asgm_bp_shotgun_prototype _returnvalue_2 "/Game/GladiatorStuff/Gladiator_BP.Gladiator_BP_C" Delay))))))))

(event Custom|Setup%20Menu%20UI
  ;[0.2351 0.6742 1] Begin Play: Add In-Game Menu Overlay Widget to the Viewport
  (bind _returnvalue (UserInterface|CreateWidget "/Game/UI/MainMenu/W_InGameMenu.W_InGameMenu_C" self))
  (bind _output_get (Variables|Default|SetW_TravelMenu _returnvalue))
  (UserInterface|Viewport|AddtoViewport _output_get 0)
  (Widget|SetVisibility _output_get "Hidden"))

(event Custom|HostSession_Event
  ;[1 1 1] Handle Sessions via Game Instance
  ;;[1 0.6539 0.3559] Send Command to Game Instance to Host Game Session
  (bind _asgi_sggprototype (Utilities|Casting|CastToGI_SGGPrototype (Game|GetGameInstance))
    (:then
      (Default|GIHostLobby _asgi_sggprototype self))
    (:CastFailed
      (Development|PrintString "Error: Cast To Game Instance Failed" true true "(R=1.000000,G=0.188499,B=0.000000,A=1.000000)"))))

(event EventBeginPlay
  ;[0.2351 0.6742 1] Begin Play: Add In-Game Menu Overlay Widget to the Viewport
  (CallFunction|SetupMenuUI)
  (CallFunction|CreateHUD))

(event EventEndPlay
  (params (EndPlayReason :type EEndPlayReason%20Enum :default "Destroyed"))
  (bind _w_travelmenu (Variables|Default|GetW_TravelMenu))
  (bind _hud (Variables|Default|GetHUD))
  ;[1 1 1] Disconnect UI to avoid crash from Player Controller that no longer exists
  (Utilities|IsValid _w_travelmenu
    (:Is%20Valid
      (Widget|RemovefromParent _w_travelmenu)
      (Utilities|IsValid _hud
        (:Is%20Valid
          (Widget|RemovefromParent _hud))))))

(event Input|ActionEvents|InputActionMenu
  (params (Key :type Key%20Structure :default "AnyKey"))
  (bind _w_travelmenu (Variables|Default|GetW_TravelMenu))
  ;[1 1 1] UI: Logic for Opening and closing In-Game Menu
  (:Pressed
    (Utilities|IsValid _w_travelmenu
      (:Is%20Valid
        (switch Utilities|FlowControl|Switch|SwitchonESlateVisibility (Widget|GetVisibility _w_travelmenu)
          (:Visible
            (CallFunction|SetinGameMenuVisibility _w_travelmenu "Hidden"))
          (:Hidden
            (CallFunction|SetinGameMenuVisibility _w_travelmenu "Visible"))))
      (:Is%20Not%20Valid
        (Development|PrintString "Error: No Assigned Menu Widget" true true "(R=1.000000,G=0.188499,B=0.000000,A=1.000000)" 2e+01)))))

(event Input|AxisEvents|InputAxisMoveForward
  (params (AxisValue :type Float%20%28single-precision%29))
  ;[0.2351 0.6742 1] Pipe Movement Logic to Controlled Pawn
  (bind _asgladiator_bp (Utilities|Casting|CastToGladiator_BP (Pawn|GetControlledPawn)))
  (Class|Gladiator|MoveForward _asgladiator_bp AxisValue))

(event Input|AxisEvents|InputAxisMoveRight
  (params (AxisValue :type Float%20%28single-precision%29))
  ;[0.2351 0.6742 1] Pipe Movement Logic to Controlled Pawn
  (bind _asgladiator_bp (Utilities|Casting|CastToGladiator_BP (Pawn|GetControlledPawn)))
  (Class|Gladiator|MoveRight _asgladiator_bp AxisValue))

(event Input|KeyboardEvents|K
  (params (Key :type Key%20Structure :default "AnyKey"))
  (:Pressed
    (CallFunction|GetListOfPlayersServer)))

(fn ConstructionScript)

(fn SetinGameMenuVisibility
  (params (WidgetReference :type Widget%20Object%20Reference) (WidgetVisibilitySetting :type ESlateVisibility%20Enum))
  (bind _self self)
  (Utilities|IsValid WidgetReference
    (:Is%20Valid
      (switch Utilities|FlowControl|Switch|SwitchonESlateVisibility WidgetVisibilitySetting
        (:Visible
          ;[1 1 1] Make Visible
          (Widget|SetVisibility WidgetReference "Visible")
          (Input|SetInputModeGameandUI _self WidgetReference false true)
          (Variables|Default|SetbShowMouseCursor true))
        (:Hidden
          ;[1 1 1] Make Hidden
          (Widget|SetVisibility WidgetReference "Hidden")
          (Input|SetInputModeGameOnly _self)
          (Variables|Default|SetbShowMouseCursor false))))
    (:Is%20Not%20Valid
      (Development|PrintString "Error: No Assigned Menu Widget" true true "(R=1.000000,G=0.188499,B=0.000000,A=1.000000)" 2e+01))))