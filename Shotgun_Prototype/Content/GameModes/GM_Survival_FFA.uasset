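; Free-for-all survival game mode that runs teamless matches where each player has a single life.
; BeginPlay sets the team and life counts before calling the parent game mode's setup.
; Every tick it reads the living-player list from GS_BP_Prototype and, while exactly one player remains, prints that player's name as the winner, with no match-end logic here.
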(event EventBeginPlay
  (Variables|Default|SetNumTeams -1)
  (Variables|Default|SetNumLives 1)
  (|CallParentFunction))

(event EventTick
  (params (DeltaSeconds :type Float%20%28single-precision%29))
  (|CallParentFunction DeltaSeconds)
  (bind _asgs_bp_prototype (Utilities|Casting|CastToGS_BP_Prototype (Game|GetGameState)))
  (if (== 1 (Utilities|Array|Length (Variables|/Game/GS_BP_Prototype.GS_BP_Prototype_C|GetLivingPlayers _asgs_bp_prototype)))
    (Development|PrintString (Utilities|String|Append (Utilities|GetDisplayName (Utilities|Array|Get(acopy) (Variables|/Game/GS_BP_Prototype.GS_BP_Prototype_C|GetLivingPlayers _asgs_bp_prototype))) " Win!"))))

(fn ConstructionScript
  (|CallParentFunction))