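; Team survival game mode that sets up two teams with one life each and watches for the last team standing.
; Every tick it reads LivingPlayers from GS_BP_Prototype and compares each player's PS_BP_Prototype team to the first one's.
; When all living players share a team, it prints that team as the winner to screen each frame, without ending the match.
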(event EventBeginPlay
  (Variables|Default|SetNumTeams 2)
  (Variables|Default|SetNumLives 1)
  (|CallParentFunction))

(event EventTick
  (params (DeltaSeconds :type Float%20%28single-precision%29))
  (|CallParentFunction DeltaSeconds)
  (bind _asgs_bp_prototype (Utilities|Casting|CastToGS_BP_Prototype (Game|GetGameState)))
  (if (> (Utilities|Array|Length (Variables|/Game/GS_BP_Prototype.GS_BP_Prototype_C|GetLivingPlayers _asgs_bp_prototype)) 0)
    (bind _asps_bp_prototype (Utilities|Casting|CastToPS_BP_Prototype (Utilities|Array|Get(acopy) (Variables|/Game/GS_BP_Prototype.GS_BP_Prototype_C|GetLivingPlayers _asgs_bp_prototype))))
    (Variables|Default|SetSingleTeam true)
    (for _array_element (Variables|/Game/GS_BP_Prototype.GS_BP_Prototype_C|GetLivingPlayers _asgs_bp_prototype)
      (bind _asps_bp_prototype_2 (Utilities|Casting|CastToPS_BP_Prototype _array_element))
      (if (not (== (Variables|/Game/PS_BP_Prototype.PS_BP_Prototype_C|GetTeam _asps_bp_prototype_2) (Variables|/Game/PS_BP_Prototype.PS_BP_Prototype_C|GetTeam _asps_bp_prototype)))
        (Variables|Default|SetSingleTeam false)))
    (if (Variables|Default|GetSingleTeam)
      (Development|PrintString (Utilities|String|Append "Team " (Utilities|String|ToString(Integer) (Variables|/Game/PS_BP_Prototype.PS_BP_Prototype_C|GetTeam _asps_bp_prototype)) " Wins!")))))

(fn ConstructionScript
  (|CallParentFunction))