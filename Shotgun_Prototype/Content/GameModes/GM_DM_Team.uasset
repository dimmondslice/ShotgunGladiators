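; Team deathmatch game mode that configures two teams and sets the lives count to -1 on BeginPlay, before calling the parent logic.
; Each Tick, it reads the match state from GS_BP_Prototype and, during Gameplay, polls every team's score.
; When any score strictly exceeds ScoreToWin, it switches the game state's match state to EndGame.
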(event EventBeginPlay
  (Variables|Default|SetNumTeams 2)
  (Variables|Default|SetNumLives -1)
  (|CallParentFunction))

(event EventTick
  (params (DeltaSeconds :type Float%20%28single-precision%29))
  (|CallParentFunction DeltaSeconds)
  (bind _asgs_bp_prototype (Utilities|Casting|CastToGS_BP_Prototype (Game|GetGameState)))
  (switch Utilities|FlowControl|Switch|SwitchonMatchState (Variables|/Game/GS_BP_Prototype.GS_BP_Prototype_C|GetMatch%20State _asgs_bp_prototype)
    (:NewEnumerator1
      (for _array_element (Variables|/Game/GS_BP_Prototype.GS_BP_Prototype_C|GetTeams _asgs_bp_prototype)
        (if (> (.Score (Utilities|Struct|BreakTeam _array_element)) (Variables|Default|GetScore%20To%20Win))
          (Default|SetMatchState _asgs_bp_prototype "NewEnumerator2"))))))

(fn ConstructionScript
  (|CallParentFunction))