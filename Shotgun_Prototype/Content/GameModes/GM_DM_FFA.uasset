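; Free-for-all deathmatch game mode that ends the match once any player's score exceeds the win threshold.
; On begin play it sets team and life counts to -1, then runs the parent mode's setup.
; During the Gameplay state, its tick scans every player state in the game state and switches the match to EndGame when a score passes ScoreToWin.
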(event Custom|ReceiveTick_Copy
  (params (DeltaSeconds :type Float%20%28single-precision%29))
  (|CallParentFunction DeltaSeconds)
  (bind _asgs_bp_prototype (Utilities|Casting|CastToGS_BP_Prototype (Game|GetGameState)))
  (switch Utilities|FlowControl|Switch|SwitchonMatchState (Variables|/Game/GS_BP_Prototype.GS_BP_Prototype_C|GetMatch%20State _asgs_bp_prototype)
    (:NewEnumerator1
      (for _array_element (Variables|/Script/Engine.GameState|GetPlayerArray _asgs_bp_prototype)
        (bind _asps_bp_prototype (Utilities|Casting|CastToPS_BP_Prototype _array_element))
        (if (> (Variables|/Game/PS_BP_Prototype.PS_BP_Prototype_C|GetPlayerScore _asps_bp_prototype) (Variables|Default|GetScore%20To%20Win))
          (Default|SetMatchState _asgs_bp_prototype "NewEnumerator2"))))))

(event EventBeginPlay
  (Variables|Default|SetNumTeams -1)
  (Variables|Default|SetNumLives -1)
  (|CallParentFunction))

(fn ConstructionScript
  (|CallParentFunction))