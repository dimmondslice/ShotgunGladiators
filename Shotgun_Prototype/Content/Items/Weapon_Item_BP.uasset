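; Gladiator weapon item that handles server-side firing, hit detection, ammo and reloading.
; Firing checks cooldown, reload state and magazine, sphere-traces along the client's view to apply point damage, then triggers gun montages, recoil camera shake and fire-rate cooldown.
; Reloading multicasts first- and third-person montages, then refills the magazine from reserve ammo after a delay.
; A multicast hit reaction, not called here, blends upper-body physics through a timeline after an impulse.
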(event Custom|ReloadWeapon
  (params (ThirdPersonMesh :type Skeletal%20Mesh%20Component%20Object%20Reference) (FirstPersonMesh :type Skeletal%20Mesh%20Component%20Object%20Reference))
  ;[1 0.6539 0.3559] Server-Side Reload Function
  (if (< (Variables|Default|GetshotsInMagazine) (Variables|Default|GetmagazineSize))
    (Variables|Default|SetisReloading true)
    (CallFunction|ReloadWeaponEffectsMulticast ThirdPersonMesh FirstPersonMesh)
    (Utilities|FlowControl|Delay (Variables|Default|GetreloadTime))
    (Variables|Default|SetisReloading false)
    (CallFunction|ReloadWeaponFunc)))

(event Custom|Destroy%20Self
  (Actor|DestroyActor))

(event Custom|ApplyShootForce_Multicast
  (params (HitActor :type Actor%20Object%20Reference) (HitComponent :type Primitive%20Component%20Object%20Reference) (HitBoneName :type Name) (ShootDirection :type Vector))
  (bind _returnvalue (Utilities|Name|MakeLiteralName "Spine1"))
  (bind _asskeletal_mesh_component (Utilities|Casting|CastToSkeletalMeshComponent HitComponent))
  (Class|SkeletalMeshComponent|SetAllBodiesBelowPhysicsBlendWeight _asskeletal_mesh_component _returnvalue 0.5 false)
  (Physics|AddImpulseatLocation _asskeletal_mesh_component (Math|Vector|Normalize ShootDirection) "0, 0, 0" HitBoneName)
  (bind _physicsblendcurve (Timeline|Timeline_0 PlayFromStart)
    (:Update
      (Class|SkeletalMeshComponent|SetAllBodiesBelowPhysicsBlendWeight _asskeletal_mesh_component _returnvalue _physicsblendcurve false))))

(event Custom|ServerFire_CapsuleTrace
  (params (ClientEyePos :type Vector) (ClientEyeRot :type Rotator) (Instigator :type Controller%20Object%20Reference))
  (bind _returnvalue (Math|Vector|GetForwardVector ClientEyeRot))
  (bind _spread (Variables|Default|Getspread))
  ;[1 0.6539 0.3559] Server-Side Logic for handling hit detection
  (bind _outhit (Class|KismetSystemLibrary|SphereTraceSingleNEW (+ ClientEyePos (* _returnvalue _spread)) (+ ClientEyePos (* _returnvalue (Variables|Default|Getrange))) _spread "TraceTypeQuery3" false (Utilities|Array|MakeArray (Pawn|GetControlledPawn Instigator)) "None" true))
  (Game|Damage|ApplyPointDamage (.HitActor (Collision|BreakHitResult _outhit)) (Variables|Default|GetbaseDamage) (* (Math|Vector|Normalize (- (.TraceEnd (Collision|BreakHitResult _outhit)) (.TraceStart (Collision|BreakHitResult _outhit)))) (Variables|Default|GetHitForce)) _outhit Instigator self (Variables|Default|GetDamageType)))

(event Custom|FireWeapon_Effects
  (params (ShootingGladiator :type Gladiator%20BP%20Object%20Reference%20%28by%20ref%29))
  (bind _shootmontage (Variables|Default|GetShootMontage))
  (Utilities|IsValid ShootingGladiator
    (:Is%20Valid
      (if (Pawn|IsLocallyControlled ShootingGladiator)
        (Animation|Montage|MontagePlay (Components|SkeletalMesh|GetAnimInstance (Variables|/Game/GladiatorStuff/Gladiator_BP.Gladiator_BP_C|GetFirstPersonGun ShootingGladiator)) _shootmontage 1.0)
        (else
          (Animation|Montage|MontagePlay (Components|SkeletalMesh|GetAnimInstance (Variables|/Game/GladiatorStuff/Gladiator_BP.Gladiator_BP_C|GetThirdPersonGun ShootingGladiator)) _shootmontage 1.0))))))

(event Custom|ActivateFirerateCooldown
  ;[1 1 1] Trigger Weapon's Firerate Cooldown (Sets Replicated Variable)
  (Variables|Default|SetisOnFireCooldown true)
  (Utilities|FlowControl|Delay (Variables|Default|GetfireRate))
  (Variables|Default|SetisOnFireCooldown false))

(event Custom|ReloadWeaponEffects_Multicast
  (params (ThirdPersonMesh :type Skeletal%20Mesh%20Component%20Object%20Reference) (FirstPersonMesh :type Skeletal%20Mesh%20Component%20Object%20Reference))
  (bind _returnvalue (Components|SkeletalMesh|GetAnimInstance FirstPersonMesh))
  (bind _returnvalue_2 (Components|SkeletalMesh|GetAnimInstance ThirdPersonMesh))
  (Utilities|FlowControl|Sequence
    (:then_0
      (Animation|Montage|MontagePlay _returnvalue_2 (Variables|Default|GetReloadMontage_ThirdPerson) 1.0)
      (bind _asgladiator_bp (Utilities|Casting|CastToGladiator_BP (Class|AnimInstance|GetOwningActor _returnvalue_2))
        (:then
          (Animation|Montage|MontagePlay (Components|SkeletalMesh|GetAnimInstance (Variables|/Game/GladiatorStuff/Gladiator_BP.Gladiator_BP_C|GetThirdPersonGun _asgladiator_bp)) (Variables|Default|GetGunReloadMontage) 1.0))
        (:CastFailed
          (Development|PrintString "failed to do the thing"))))
    (:then_1
      (Animation|Montage|MontagePlay _returnvalue (Variables|Default|GetReloadMontage_FirstPerson) 1.0)
      (bind _asgladiator_bp_2 (Utilities|Casting|CastToGladiator_BP (Class|AnimInstance|GetOwningActor _returnvalue)))
      (Animation|Montage|MontagePlay (Components|SkeletalMesh|GetAnimInstance (Variables|/Game/GladiatorStuff/Gladiator_BP.Gladiator_BP_C|GetFirstPersonGun _asgladiator_bp_2)) (Variables|Default|GetGunReloadMontage) 1.0))))

(event Custom|FireWeapon
  (params (Origin :type Vector) (Rotation :type Rotator) (Instigator :type Controller%20Object%20Reference))
  (bind _returnvalue (Pawn|GetControlledPawn Instigator))
  ;[1 0.6539 0.3559] Server-Side Fire Weapon
  (if (not (Variables|Default|GetisOnFireCooldown))
    (if (not (Variables|Default|GetisReloading))
      (if (> (Variables|Default|GetshotsInMagazine) 0)
        (CallFunction|ReduceAmmo)
        (CallFunction|ServerFireCapsuleTrace Origin Rotation Instigator)
        (Utilities|IsValid _returnvalue
          (:Is%20Valid
            (bind _asgladiator_bp (Utilities|Casting|CastToGladiator_BP _returnvalue))
            (Utilities|FlowControl|Sequence
              (:then_0
                (CallFunction|FireWeaponEffects _asgladiator_bp))
              (:then_1
                (bind _asplayer_controller (Utilities|Casting|CastToPlayerController (Components|GetOwner _asgladiator_bp)))
                (Class|PlayerController|ClientPlayCameraShake _asplayer_controller (Variables|Default|GetRecoilShakeType) 1.0 "CameraLocal" "0, 0, 0"))
              (:then_2
                (CallFunction|ActivateFirerateCooldown)))))))))

(event EventTick
  (params (DeltaSeconds :type Float%20%28single-precision%29)))

(fn ConstructionScript)

(fn ReduceAmmo
  (bind _shotsinmagazine (Variables|Default|GetshotsInMagazine))
  (if (> _shotsinmagazine 0)
    (Math|Integer|DecrementInt _shotsinmagazine
      (:%20%20
        (return)))))

(fn ReloadWeaponFunc
  (bind _output_get (LocalVariables|SetRoomInMag (- (Variables|Default|GetmagazineSize) (Variables|Default|GetshotsInMagazine))))
  ;[1 1 1] If we have enough ammo to fully refil, do it
  (if (>= (Variables|Default|GetcurrentAmmo) _output_get)
    ;;[1 1 1] Reduce Current Ammo
    (Variables|Default|SetcurrentAmmo (- (Variables|Default|GetcurrentAmmo) _output_get))
    ;;[1 1 1] Fill Magazine
    (Variables|Default|SetshotsInMagazine (+ (Variables|Default|GetshotsInMagazine) _output_get))
    (else
      ;[1 1 1] If we don't have enough ammo to fully refill, dump in what we have and set current ammo to 0
      (Variables|Default|SetshotsInMagazine (+ (Variables|Default|GetshotsInMagazine) (Variables|Default|GetcurrentAmmo)))
      (Variables|Default|SetcurrentAmmo 0)))
  (return))

(fn OnRepHasOwner)