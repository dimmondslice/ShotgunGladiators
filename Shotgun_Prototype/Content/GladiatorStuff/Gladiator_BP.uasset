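; Networked first-person Gladiator character for a shotgun prototype, with gun, spawned shield, dodge sound, health and HUD.
; Input forwards firing and shielding through network events, with the held weapon handling fire and reload and the shield blocking shooting while up.
; Lethal damage sends score to the game mode and requests respawn from the controller; destruction cleans up weapon, HUD and possession.
; Tick sends a signed velocity-to-facing angle to the server for animation.
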(event BeginDodgeEvent(Dodge)
  ;[1 1 1] Dodge Sound Effect
  (CallFunction|DodgeEffectsForwardServer))

(event Custom|NetworkedShieldUp_Event
  (params (ButtonIsDown :type Boolean))
  (bind _returnvalue (Transformation|GetActorRotation))
  (bind _self self)
  ;[1 1 1] Networked Shielding, Boys
  (if ButtonIsDown ; If we want to put the shield up or down
    (if (Variables|Default|GetCanShield)
      (if (not (Variables|Default|GetShieldIsUp))
        (Variables|Default|SetCanShoot false)
        (Variables|Default|SetCanShield false)
        (Utilities|FlowControl|Delay 0.1)
        (Variables|Default|SetShieldIsUp true)
        (bind _returnvalue_2 (Game|SpawnActorfromClass "/Game/Shield.Shield_C" (Math|Transform|MakeTransform (+ (Transformation|GetActorLocation) (* (Math|Vector|GetForwardVector _returnvalue) (Variables|Default|GetShield%20Distance))) _returnvalue) "AlwaysSpawn" _self 0))
        (bind _output_get (Variables|Default|SetShield _returnvalue_2))
        (Class|Actor|AttachRootComponenttoActor _output_get _self "None" "KeepWorldPosition" true)
        (Development|PrintString "Spawned and attached shield")))
    (else
      (Utilities|FlowControl|Delay 0.18)
      (if (Variables|Default|GetShieldIsUp)
        (Variables|Default|SetCanShield true)
        (Variables|Default|SetShieldIsUp false)
        (Variables|Default|SetCanShoot true)
        (Actor|DestroyActor _returnvalue_2)
        (Variables|Default|SetShield 0)))))

(event Custom|Create%20HUD
  ;[0.2351 0.6742 1] Create HUD
  (bind _returnvalue (UserInterface|CreateWidget "/Game/UI/InGameHud/HUD.HUD_C" (Game|GetPlayerController 0)))
  (bind _output_get (Variables|Default|SetHUD _returnvalue))
  (UserInterface|Viewport|AddtoViewport _output_get 0))

(event Custom|DisconnectFromController
  (bind _returnvalue (Pawn|GetController))
  ;[1 1 1] Disconnect from the Controller when Destroyed
  (Utilities|IsValid _returnvalue
    (:Is%20Valid
      (Pawn|UnPossess _returnvalue))))

(event Custom|DropItem
  (bind _heldweapon (Variables|Default|GetHeldWeapon))
  ;[1 1 1] Destroy Item when Pawn gets Destroyed (don't worry, the variable reference is replicated)
  (Networking|SwitchHasAuthority
    (:Authority
      (Utilities|IsValid _heldweapon
        (:Is%20Valid
          (Default|DestroySelf _heldweapon))
        (:Is%20Not%20Valid
          (Development|PrintString "Failed To Destroy Weapon" true true "(R=1.000000,G=0.025834,B=0.905649,A=1.000000)" 1e+01))))))

(event Custom|SendLocalRotation_Clients
  (params (LocalCamRotation :type Rotator))
  ;[1 1 1] Animation - Record info for leaning forward and backward
  (if (Ability|HasAuthority (Game|GetGameMode))
    (Variables|Default|SetCameraLocalRotation LocalCamRotation)))

(event Custom|GetLocalRotation_Client
  ;[1 1 1] Animation - Record info for leaning forward and backward
  (CallFunction|SendLocalRotationServer (Variables|/Script/Engine.SceneComponent|GetRelativeRotation (Variables|Default|GetFirstPersonCameraComponent))))

(event Custom|BindItem
  (params (Item :type Weapon%20Item%20BP%20Class%20Reference) (ItemBindSocket :type Name) (PawnSkelMesh :type Mesh%20Component%20Object%20Reference) (PawnGripSocket :type Name))
  (Networking|SwitchHasAuthority
    (:Authority
      (bind _returnvalue (Game|SpawnActorfromClass Item (Transformation|GetSocketTransform PawnSkelMesh PawnGripSocket "RTS_World") "Undefined" 0 0))
      (bind _output_get (Variables|Default|SetHeldWeapon _returnvalue))
      (Class|Actor|AttachRootComponentto _output_get PawnSkelMesh PawnGripSocket "SnapToTarget" true))))

(event Custom|DodgeEffects_ForwardServer
  ;[1 1 1] Dodge Sound Effect
  (CallFunction|DodgeEffectsForwardMulticast))

(event Custom|UseGun_Server
  (params (ShootOrigin :type Vector) (ShootDirection :type Rotator))
  (bind _heldweapon (Variables|Default|GetHeldWeapon))
  ;[1 0.6539 0.3559] Fire and Reloading Gun
  (Utilities|IsValid _heldweapon
    (:Is%20Valid
      (Default|FireWeapon _heldweapon ShootOrigin ShootDirection (Pawn|GetController)))))

(event Custom|SendLocalRotation_Server
  (params (LocalCamRot :type Rotator))
  ;[1 1 1] Animation - Record info for leaning forward and backward
  (Networking|SwitchHasAuthority
    (:Authority
      (bind _output_get (Variables|Default|SetCameraLocalRotation LocalCamRot)))))

(event Custom|DodgeEffects_ForwardMulticast
  ;[1 1 1] Dodge Sound Effect
  (Audio|PlaySoundatLocation (Variables|Default|GetRocketDodgeSoundCue) (.Location (Math|Transform|BreakTransform (Transformation|GetSocketTransform (Variables|Character|GetMesh) "Root_Socket" "RTS_World")))))

(event Custom|Forward_DestroyHUD
  ;[0.2351 0.6742 1] Destroy Hud when Destroyed
  (CallFunction|DestroyHUD))

(event Custom|AddScore_ForwardToServer
  (params (DamageCauser :type Controller%20Object%20Reference))
  ;[1 0.6539 0.3559] Forward the call to add Score to the Server
  (bind _asgm_bp_shotgun_prototype (Utilities|Casting|CastToGM_BP_ShotgunPrototype (Game|GetGameMode)))
  (Default|AddScore _asgm_bp_shotgun_prototype DamageCauser))

(event Custom|DestroyHUD
  (bind _hud (Variables|Default|GetHUD))
  ;[0.2351 0.6742 1] Destroy HUD
  (Utilities|IsValid _hud
    (:Is%20Valid
      (Widget|RemovefromParent _hud))))

(event Custom|ReloadGun_ForwardToServer
  (CallFunction|ReloadGunServer (Variables|Character|GetMesh) (Variables|Default|GetMesh1P)))

(event Custom|GetAimToFeetAngle_Client
  (bind _returnvalue (Transformation|GetActorForwardVector))
  (bind _returnvalue_2 (Transformation|GetVelocity))
  (bind _returnvalue_3 (Math|Vector|Normalize _returnvalue_2))
  ;[1 1 1] Animation - Record info for rotating side-to-side
  ;;[1 1 1] Use Plane to determine left or right to walk
  (bind _returnvalue_4 (Class|ShotgunGladiatorsQualityOfLifeBP|MakeFPlaneNormandLoc "0, 0, 0" (Math|Vector|RotateVector _returnvalue "0,90.000000,0.000000")))
  (bind _returnvalue_5 (Class|ShotgunGladiatorsQualityOfLifeBP|PlaneDotProduct _returnvalue_4 _returnvalue_3))
  (CallFunction|SendAimtoFeetAngleServer (Math|Conversions|ToFloat(Integer) (Math|Float|Round (* (Math|Float|Sign(Float) _returnvalue_5) (Class|KismetMathLibrary|DegAcos (Math|Vector|DotProduct _returnvalue_3 (Math|Vector|Normalize _returnvalue))))))))

(event Custom|SendAimToFeetAngle_Server
  (params (AimToFeetAngle :type Float%20%28single-precision%29))
  ;[1 1 1] Animation - Record info for rotating side-to-side
  (Networking|SwitchHasAuthority
    (:Authority
      (bind _output_get (Variables|Default|SetAimToFeetAngle AimToFeetAngle)))))

(event Custom|ReloadGun_Server
  (params (ThirdPersonMesh :type Skeletal%20Mesh%20Component%20Object%20Reference) (FirstPersonMesh :type Skeletal%20Mesh%20Component%20Object%20Reference))
  (bind _heldweapon (Variables|Default|GetHeldWeapon))
  ;[1 0.6539 0.3559] Fire and Reloading Gun
  (Utilities|IsValid _heldweapon
    (:Is%20Valid
      (Default|ReloadWeapon _heldweapon ThirdPersonMesh FirstPersonMesh))))

(event Game|Damage|EventAnyDamage
  (params (Damage :type Float%20%28single-precision%29) (DamageType :type Damage%20Type%20Object%20Reference) (InstigatedBy :type Controller%20Object%20Reference) (DamageCauser :type Actor%20Object%20Reference))
  ;[1 1 1] Receive Damage
  (Variables|Default|SetHealth (- (Variables|Default|GetHealth) Damage))
  (Development|PrintString "Damaged")
  (if (<= (Variables|Default|GetHealth) 0.0)
    (Development|PrintString "dead")
    (CallFunction|AddScoreForwardtoServer InstigatedBy)
    (bind _aspc_bp_prototype (Utilities|Casting|CastToPC_BP_Prototype (Pawn|GetController self)))
    (Default|RespawnPlayer _aspc_bp_prototype true)))

(event EventTick
  (params (DeltaSeconds :type Float%20%28single-precision%29))
  (CallFunction|GetAimtoFeetAngleClient))

(event EventBeginPlay
  ;[1 1 1] Disconnect from the Controller when Destroyed
  (EventDispatchers|BindEventtoOnDestroyed (delegate Custom|DisconnectFromController))
  ;[0.2351 0.6742 1] Bind Item to Mesh
  (CallFunction|BindItem "/Game/Items/DoubleBarrel/DoubleBarrel_Weapon_Item_BP.DoubleBarrel_Weapon_Item_BP_C" "GripPoint" (Variables|Default|GetMesh1P) "GripPoint")
  (EventDispatchers|BindEventtoOnDestroyed (delegate Custom|DropItem))
  ;[0.2351 0.6742 1] Call Creation of HUD
  (CallFunction|CreateHUD)
  ;[0.2351 0.6742 1] Destroy Hud when Destroyed
  (EventDispatchers|BindEventtoOnDestroyed (delegate Custom|Forward_DestroyHUD))
  (Variables|Default|SetAimForwardVec (Transformation|GetActorForwardVector)))

(event Input|ActionEvents|InputActionFire
  (params (Key :type Key%20Structure :default "AnyKey"))
  (bind _firstpersoncameracomponent (Variables|Default|GetFirstPersonCameraComponent))
  (bind _returnvalue (Transformation|GetWorldTransform _firstpersoncameracomponent))
  (bind (_location _rotation) (Math|Transform|BreakTransform _returnvalue))
  ;[1 1 1] Shooting -> Send to Server to be handled
  (:Pressed
    (if (Variables|Default|GetCanShoot)
      (CallFunction|UseGunServer _location _rotation)
      (Animation|Montage|MontagePlay (Components|SkeletalMesh|GetAnimInstance (Variables|Default|GetMesh1P)) "/Game/Rigs/FirstPersonArms/FirstPersonFire_Montage.FirstPersonFire_Montage" 1.0)
      (bind _asgm_bp_shotgun_prototype (Utilities|Casting|CastToGM_BP_ShotgunPrototype (Game|GetGameMode)))
      (Default|PlayerShot _asgm_bp_shotgun_prototype))))

(event Input|ActionEvents|InputActionShield
  (params (Key :type Key%20Structure :default "AnyKey"))
  ;[1 1 1] Networked Shielding, Boys
  (:Pressed
    (CallFunction|NetworkedShieldUpEvent true))
  (:Released
    (CallFunction|NetworkedShieldUpEvent false)))

(fn ConstructionScript)

(fn OnRepCurrentAmmo
  (Development|PrintString "Used Ammo"))

(fn SetUpperBodyState)