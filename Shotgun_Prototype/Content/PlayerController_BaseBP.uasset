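; Base player controller that serves as the entry point for multiplayer session actions in the SGG prototype.
; Custom events for hosting, finding, joining and exiting sessions cast the Game Instance to GI_SGGPrototype and forward the request to its lobby and session functions, passing the controller itself.
; Join also passes the selected session and player name, and all four events share one error print when the cast fails.
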(event Custom|JoinSession_Event
  (params (SelectedSession :type Blueprint%20Session%20Result%20Structure) (Player%20Name :type String))
  ;[1 1 1] Handle Sessions via Game Instance
  ;;[1 0.6539 0.3559] Send Command to Game Instance to Join an Available Session
  (bind _asgi_sggprototype (Utilities|Casting|CastToGI_SGGPrototype (Game|GetGameInstance))
    (:then
      (Default|GIJoinLobby _asgi_sggprototype self SelectedSession Player%20Name))
    (:CastFailed
      (Development|PrintString "Error: Cast To Game Instance Failed" true true "(R=1.000000,G=0.188499,B=0.000000,A=1.000000)"))))

(event Custom|ExitSession_Event
  ;[1 1 1] Handle Sessions via Game Instance
  (bind _asgi_sggprototype (Utilities|Casting|CastToGI_SGGPrototype (Game|GetGameInstance))
    (:then
      (Default|GIExitSession _asgi_sggprototype self))
    (:CastFailed
      (Development|PrintString "Error: Cast To Game Instance Failed" true true "(R=1.000000,G=0.188499,B=0.000000,A=1.000000)"))))

(event Custom|FindSessions_Event
  ;[1 1 1] Handle Sessions via Game Instance
  ;;[1 1 1] Send Command to Game Instance to FInd Available Sessions
  (bind _asgi_sggprototype (Utilities|Casting|CastToGI_SGGPrototype (Game|GetGameInstance))
    (:then
      (Default|GIFindLobbies _asgi_sggprototype self))
    (:CastFailed
      (Development|PrintString "Error: Cast To Game Instance Failed" true true "(R=1.000000,G=0.188499,B=0.000000,A=1.000000)"))))

(event Custom|HostSession_Event
  ;[1 1 1] Handle Sessions via Game Instance
  ;;[1 0.6539 0.3559] Send Command to Game Instance to Host Game Session
  (bind _asgi_sggprototype (Utilities|Casting|CastToGI_SGGPrototype (Game|GetGameInstance))
    (:then
      (Default|GIHostLobby _asgi_sggprototype self "None"))
    (:CastFailed
      (Development|PrintString "Error: Cast To Game Instance Failed" true true "(R=1.000000,G=0.188499,B=0.000000,A=1.000000)"))))

(event EventBeginPlay)

(event EventTick
  (params (DeltaSeconds :type Float%20%28single-precision%29)))

(fn ConstructionScript)